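; BP_SideCharacter is a slime character with flipbook movement animation and a directional dash.
; UpdataAnimation picks the flipbook by death, then dash, then walk direction, favoring horizontal and keeping the last facing when idle; the death slot is empty.
; Dash launches the slime along its input direction, makes noise, and blocks input until a short retriggerable delay ends.
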(event EventUpdataAnimation
  ;[1 0.04957 0.1995] Updata_Aniation
  (if (Variables|Default|GetbDeath)
    (Variables|Default|SetAnimSet 3) ; death
    (elif (Variables|Default|GetbDash)
      (Variables|Default|SetAnimSet 4) ; dash
      (else
        (CallFunction|SetAnimWalk))))
  (Sprite|SetFlipbook (Variables|Default|GetSprite) (Utilities|Select :Index (Variables|Default|GetAnimSet) :Option%200 "/Game/Characters/Filpbook/Slime_Dowmwalk.Slime_Dowmwalk" :Option%201 "/Game/Characters/Filpbook/Slime_Topwalk.Slime_Topwalk" :Option%202 "/Game/Characters/Filpbook/Slime_R_Move.Slime_R_Move" :Option%203 0 :Option%204 "/Game/Characters/Filpbook/Slime_Dash.Slime_Dash")))

(event EventDash
  ;[0.4728 0.4172 1] Dash
  (if (or (!= (Variables|Default|GetDirectionUp) 0.0) (!= (Variables|Default|GetDirectionRight) 0.0))
    (Variables|Default|SetbDash true)
    (Class|Actor|MakeNoise 1.0 0 (Transformation|GetActorLocation) 0.0 "None") ; 製造噪音
    (Input|DisableInput 0)
    (Character|LaunchCharacter (* (Math|Vector|MakeVector (Variables|Default|GetDirectionRight) (Variables|Default|GetDirectionUp) 0.0) 2000) false false)
    (Utilities|FlowControl|RetriggerableDelay 0.25)
    (Variables|Default|SetbDash false)
    (Input|EnableInput 0)))

(fn ConstructionScript)

(fn SetAnimWalk
  (if (!= (Variables|Default|GetDirectionRight) 0.0) ; 左右優先
    (Variables|Default|SetAnimSet 2)
    (Variables|Default|SetWalkSet 2)
    (elif (!= (Variables|Default|GetDirectionUp) 0.0)
      (if (> (Variables|Default|GetDirectionUp) 0.0) ; 下上
        (Variables|Default|SetAnimSet 0)
        (Variables|Default|SetWalkSet 0)
        (else
          (Variables|Default|SetAnimSet 1)
          (Variables|Default|SetWalkSet 1)))
      (else
        (Variables|Default|SetAnimSet (Variables|Default|GetWalkSet)))))
  (return))